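; Base pickup actor that hands itself to an overlapping character and then destroys itself.
; On sphere overlap it gets the character through a GetCharacterRef message and requires that it can be damaged and is not already holding an item.
; A DoOnce limits the GivePlayerPickup handoff to a single trigger.
; The construction script applies the Mesh variable to the pickup mesh, and the pickup's own GetCharacterRef is empty.
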(event OnComponentBeginOverlap(PickupSphere)
  (params (OverlappedComponent :type Primitive%20Component%20Object%20Reference) (OtherActor :type Actor%20Object%20Reference) (OtherComp :type Primitive%20Component%20Object%20Reference) (OtherBodyIndex :type Integer) (bFromSweep :type Boolean) (SweepResult :type Hit%20Result%20Structure%20%28by%20ref%29))
  (bind _ref (Class|BPIPlayer|GetCharacterRef(Message) OtherActor))
  (if (Variables|/Script/Engine.Actor|GetbCanBeDamaged _ref)
    (if (not (Variables|/Game/Tech/Blueprints/BP_BaseCharacter.BP_BaseCharacter_C|GetIsPlayerHoldingItem? _ref))
      (Utilities|FlowControl|DoOnce false
        (:Completed
          (Default|GivePlayerPickup _ref self)
          (Actor|DestroyActor))))))

(fn ConstructionScript
  (Components|StaticMesh|SetStaticMesh (Variables|Default|GetPickupMesh) (Variables|Default|GetMesh)))

(fn GetCharacterRef
  (return 0))