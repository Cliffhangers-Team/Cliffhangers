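; BP_IceBarrel is a trap that freezes pawns caught in its blast.
; An overlap on DetectionBox starts a timer of TrapActionTime, which then fires the Explode event.
; Explode runs a multi-sphere trace for pawns at the FireArrow location, with debug drawing left on, and sends FreezePlayerMessage with a fixed duration to each hit actor.
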(event OnComponentBeginOverlap(DetectionBox)
  (params (OverlappedComponent :type Primitive%20Component%20Object%20Reference) (OtherActor :type Actor%20Object%20Reference) (OtherComp :type Primitive%20Component%20Object%20Reference) (OtherBodyIndex :type Integer) (bFromSweep :type Boolean) (SweepResult :type Hit%20Result%20Structure%20%28by%20ref%29))
  (Utilities|Time|SetTimerbyEvent (delegate Custom|Explode) (Variables|Default|GetTrapActionTime)))

(event Custom|Explode
  (bind _firearrow (Variables|Default|GetFireArrow))
  (bind _returnvalue (Transformation|GetWorldLocation _firearrow))
  (bind (_outhits _returnvalue_2) (Collision|MultiSphereTraceForObjects _returnvalue _returnvalue 4e+02 (Utilities|Array|MakeArray "ObjectTypeQuery3") true 0 "ForDuration"))
  (if _returnvalue_2
    (for _array_element _outhits
      (Class|BPIPlayer|FreezePlayer(Message) (.HitActor (Collision|BreakHitResult _array_element)) 4.0))))

(fn ConstructionScript
  (|CallParentFunction))

(fn GetCharacterRef
  (return 0))