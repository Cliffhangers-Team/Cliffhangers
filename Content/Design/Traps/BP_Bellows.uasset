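; BP_Bellows is a trap that launches nearby pawns when something overlaps its DetectionBox.
; The overlap runs a pawn box trace at DamageBox, oriented to the Cube and ignoring the triggering actor, with debug drawing on.
; Each hit's character, fetched by GetCharacterRef message, is launched along the Direction component's forward vector with upward lift.
; BellowsCooldown is cleared without any delay.
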(event OnComponentBeginOverlap(DetectionBox)
  (params (OverlappedComponent :type Primitive%20Component%20Object%20Reference) (OtherActor :type Actor%20Object%20Reference) (OtherComp :type Primitive%20Component%20Object%20Reference) (OtherBodyIndex :type Integer) (bFromSweep :type Boolean) (SweepResult :type Hit%20Result%20Structure%20%28by%20ref%29))
  (bind _damagebox (Variables|Default|GetDamageBox))
  (bind _returnvalue (Transformation|GetWorldLocation _damagebox))
  (if (not (Variables|Default|GetBellowsCooldown))
    (Variables|Default|SetBellowsCooldown true)
    (bind (_outhits _returnvalue_2) (Class|KismetSystemLibrary|BoxTraceMultiforObjects _returnvalue _returnvalue "150.000000,300.000000,50.000000" (Transformation|GetWorldRotation (Variables|Default|GetCube)) (Utilities|Array|MakeArray "ObjectTypeQuery3") false (Utilities|Array|MakeArray OtherActor) "ForDuration" true))
    (if _returnvalue_2
      (for _array_element _outhits
        (bind _ref (Class|BPIPlayer|GetCharacterRef(Message) (.HitActor (Collision|BreakHitResult _array_element))))
        (Character|LaunchCharacter _ref (+ (* (Math|Vector|GetForwardVector (Variables|Default|GetDirection)) 1.5e+03) "0.000000,0.000000,350.000000") false true)))
    (Variables|Default|SetBellowsCooldown false)))

(event OnComponentBeginOverlap(DamageBox)
  (params (OverlappedComponent :type Primitive%20Component%20Object%20Reference) (OtherActor :type Actor%20Object%20Reference) (OtherComp :type Primitive%20Component%20Object%20Reference) (OtherBodyIndex :type Integer) (bFromSweep :type Boolean) (SweepResult :type Hit%20Result%20Structure%20%28by%20ref%29)))

(fn ConstructionScript
  (|CallParentFunction))

(fn GetCharacterRef
  (return 0))