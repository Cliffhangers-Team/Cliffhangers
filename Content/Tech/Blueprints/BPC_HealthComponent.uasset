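; Actor component that tracks health and handles damage and death for its owner.
; BeginPlay resets health to maximum and enables damage through SetValuesToDefaults.
; ApplyDamage subtracts damage while CanBeDamaged is true, clamps health between zero and maximum, and calls Death at zero.
; Death disables further damage and only prints a debug message, and a disconnected DoOnce remains as a noted alternative to the boolean guard.
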(event Custom|ApplyDamage
  (params (Damage :type Integer))
  (if (Variables|Default|GetCanBeDamaged?)
    (bind _output_get (Variables|Default|SetCurrentHealth (Math|Integer|Clamp(Integer) (- (Variables|Default|GetCurrentHealth) Damage) 0 (Variables|Default|GetMaxHealth))))
    (if (<= _output_get 0)
      (CallFunction|Death))))

(event Custom|Death
  (Variables|Default|SetCanBeDamaged? false)
  (Development|PrintString "Dead"))

(event EventBeginPlay
  (CallFunction|SetValuestoDefaults))

(fn SetValuestoDefaults
  (Variables|Default|SetCurrentHealth (Variables|Default|GetMaxHealth))
  (Variables|Default|SetCanBeDamaged? true))